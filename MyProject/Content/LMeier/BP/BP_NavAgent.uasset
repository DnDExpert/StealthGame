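; BP_NavAgent is a patrolling AI enemy that walks a looping list of nav points and chases the player when spotted.
; AI perception of the "Player"-tagged actor toggles Seen, which Tick uses to switch between fast pursuit and slow patrol.
; Overlapping a nav point advances the route after a retriggerable delay.
; Projectile hits report the kill to the game mode and destroy it, while capsule contact with the player shows end-game widgets and pauses.
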(event `self.ReceiveTick`
  (params (DeltaSeconds :type "Float (single-precision)"))
  (bind _charactermovement (`self.CharacterMovement`))
  (bind _returnvalue (`AIBlueprintHelperLibrary.GetAIController` (`self.GetOwner`)))
  ;[1 1 1] Patrol Script
  (if (`self.Seen`)
    (set `CharacterMovementComponent.MaxWalkSpeed` 600.0 _charactermovement)
    (`AIBlueprintHelperLibrary.SimpleMoveToActor` _returnvalue (`self.PlayerRef`))
    (else
      (set `CharacterMovementComponent.MaxWalkSpeed` 200.0 _charactermovement)
      (bind _currentnavpoint (`self.GetCurrentNavPoint`))
      (`AIBlueprintHelperLibrary.SimpleMoveToActor` _returnvalue _currentnavpoint :!label _label))))

(event `self.ReceiveActorBeginOverlap`
  (params (OtherActor :type "Actor Object Reference"))
  ;[1 1 1] Patrol Script
  (if (== (`GameplayStatics.GetObjectClass` OtherActor) "/Game/FirstPersonBP/Blueprints/FirstPersonProjectile.FirstPersonProjectile_C")
    (bind _asfirst_person_game_mode (cast `/Game/FirstPersonBP/Blueprints/FirstPersonGameMode` (`GameplayStatics.GetGameMode`)))
    (`/Game/FirstPersonBP/Blueprints/FirstPersonGameMode.PatrolKilled` _asfirst_person_game_mode)
    (`self.K2_DestroyActor`)
    (elif (== (`GameplayStatics.GetObjectClass` OtherActor) "/Game/LMeier/BP/BP_NavPoint.BP_NavPoint_C")
      (`KismetSystemLibrary.RetriggerableDelay` 3.0)
      (`self.ChooseNextNavPoint`)
      (goto _label))))

(event `self.AIPerception.OnTargetPerceptionUpdated`
  (params (Actor :type "Actor Object Reference") (Stimulus :type "AIStimulus Structure"))
  (if (`self.ActorHasTag` Actor "Player")
    (if (`.bSuccessfullySensed` (break `AIStimulus` Stimulus))
      (set `self.Seen` true)
      (else
        (set `self.Seen` false)))))

(event `self.Capsule.OnComponentBeginOverlap`
  (params (OverlappedComponent :type "PrimitiveComponent Object Reference") (OtherActor :type "Actor Object Reference") (OtherComp :type "PrimitiveComponent Object Reference") (OtherBodyIndex :type Integer) (bFromSweep :type Boolean) (SweepResult :type "HitResult Structure (by ref)"))
  (cast `/Game/FirstPersonBP/Blueprints/FirstPersonCharacter` OtherActor)
  (bind _returnvalue (`|CreateWidget` "/Game/LMeier/BP/W_EndGame.W_EndGame_C"))
  (bind _returnvalue_2 (`|CreateWidget` "/Game/LMeier/BP/W_Caught.W_Caught_C"))
  (`UserWidget.AddToViewport` _returnvalue 0)
  (`UserWidget.AddToViewport` _returnvalue_2 0)
  (`GameplayStatics.SetGamePaused` true))

(fn `ChooseNextNavPoint`
  (bind _result (`/Engine/EditorBlueprintResources/StandardMacros.IncrementInt` (`self.Selected Index`))
    (:`  `
      (bind _output_get (set `self.Selected Index` _result))
      (if (not (`KismetArrayLibrary.Array_IsValidIndex` (`self.myNavpoints`) _output_get))
        (set `self.Selected Index` 0)))))

(fn `GetCurrentNavPoint`
  (returns (CurrentNavPoint :type "/Game/LMeier/BP/BP_NavPoint Object Reference"))
  (bind _output (`|GetArrayItem` (`self.myNavpoints`) (`self.Selected Index`)))
  (`/Engine/EditorBlueprintResources/StandardMacros.IsValid` _output
    (:`Is Valid`
      _)
    (:`Is Not Valid`
      (`KismetSystemLibrary.PrintString` (`KismetStringLibrary.Concat_StrStr` (`KismetSystemLibrary.GetDisplayName` (`self.GetOwner`)) " Just tried to access an invalid nav point, make sure the patrol component has these assigned in the level editor") true true (struct :`R` 1.0 :`A` 1.0) 10.0)))
  (return _output))

(fn `UserConstructionScript`)